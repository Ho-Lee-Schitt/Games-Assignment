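; Default_Player is the golf game's player actor, handling touch aiming, the camera and ball turnover between shots.
; Horizontal drags yaw the ball's spring arm and snap the player to the ball's camera; during a shot the camera only rotates to track it.
; When the ball stops, a replacement spawns facing the hole; NewBall(true) respawns it at LastPosition instead, and both refresh the Club's reference.
; Tick logic halts once GameController is Complete.
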(event Custom|MoveCamera
  (Transformation|SetActorLocation (Transformation|GetWorldLocation (Variables|/Game/Blueprints/Golf_Ball_BP.Golf_Ball_BP_C|GetCamera (Variables|Default|GetGolfBall))) false false)
  (CallFunction|LookatBall))

(event Custom|NewBall
  (params (Destroyed? :type Boolean))
  (if Destroyed?
    (bind _returnvalue (Game|SpawnActorfromClass "/Game/Blueprints/Golf_Ball_BP.Golf_Ball_BP_C" (Math|Transform|MakeTransform (.location (Variables|/Script/GameAssignment.Golf_Ball|GetLastPosition (Variables|Default|GetGolfBall))) (.rotation (Variables|/Script/GameAssignment.Golf_Ball|GetLastPosition (Variables|Default|GetGolfBall))) "1,1,1") "Undefined" 0 0))
    (Actor|DestroyActor (Variables|Default|GetGolfBall))
    (Variables|Default|SetGolfBall _returnvalue)
    (else
      (bind _returnvalue_2 (Game|SpawnActorfromClass "/Game/Blueprints/Golf_Ball_BP.Golf_Ball_BP_C" (Math|Transform|MakeTransform (.location (Transformation|GetWorldTransform (Variables|/Script/GameAssignment.Golf_Ball|GetBall (Variables|Default|GetGolfBall)))) (Math|Rotator|MakeRotator 0.0 0.0 (.yaw (Math|Rotator|FindLookatRotation (Transformation|GetWorldLocation (Variables|/Game/Blueprints/Golf_Ball_BP.Golf_Ball_BP_C|GetSpringArmComponentLine (Variables|Default|GetGolfBall))) (.location (Transformation|GetActorTransform (Variables|Default|GetHole)))))) "1,1,1") "Undefined" 0 0))
      (Development|PrintString "Destroying Ball")
      (Actor|DestroyActor (Variables|Default|GetGolfBall))
      (Variables|Default|SetGolfBall _returnvalue_2)))
  (Class|Club|GetGolfBall (Variables|Default|GetClub))
  (Variables|Default|SetGameState "NewEnumerator0")
  (CallFunction|MoveCamera)
  (CallFunction|LookatBall))

(event Custom|LookAtBall
  (bind _camera (Variables|Default|GetCamera))
  (bind _output_get (Variables|Default|SetLookAt (Transformation|GetActorLocation (Variables|Default|GetGolfBall))))
  (Transformation|SetWorldRotation _camera (Math|Rotator|FindLookatRotation (Math|Transform|TransformLocation (Transformation|GetWorldTransform _camera) "0, 0, 0") _output_get) false false))

(event EventBeginPlay
  (bind _outactors (Actor|GetAllActorsOfClass "/Game/Blueprints/Golf_Ball_BP.Golf_Ball_BP_C"))
  (for _array_element _outactors
    (Variables|Default|SetGolfBall _array_element))
  (Variables|Default|SetGameState "NewEnumerator0")
  (Development|PrintString "Ball Rest")
  (CallFunction|MoveCamera)
  (CallFunction|LookatBall)
  (bind _outactors_2 (Actor|GetAllActorswithTag "Hole"))
  (for _array_element_2 _outactors_2
    (Variables|Default|SetHole _array_element_2))
  (bind _outactors_3 (Actor|GetAllActorsOfClass "/Game/Blueprints/GameController_BP.GameController_BP_C"))
  (for _array_element_3 _outactors_3
    (Variables|Default|SetGameController _array_element_3)))

(event Collision|EventActorBeginOverlap
  (params (OtherActor :type Actor%20Object%20Reference)))

(event EventTick
  (params (DeltaSeconds :type Float%20%28single-precision%29))
  (bind _returnvalue (Game|GetPlayerController 0))
  (bind _finger (Variables|Default|GetFinger))
  (bind _golfball (Variables|Default|GetGolfBall))
  (bind (_locationx _locationy _biscurrentlypressed) (Class|PlayerController|GetInputTouchState _returnvalue _finger))
  (bind _springarmcomponentline (Variables|/Game/Blueprints/Golf_Ball_BP.Golf_Ball_BP_C|GetSpringArmComponentLine _golfball))
  (bind _relativerotation (Variables|/Script/Engine.SceneComponent|GetRelativeRotation _springarmcomponentline))
  (if (not (Variables|/Game/Blueprints/GameController_BP.GameController_BP_C|GetComplete (Variables|Default|GetGameController)))
    (if (Variables|/Script/GameAssignment.Golf_Ball|GetBallMoving (Variables|Default|GetGolfBall))
      (if (Utilities|Enum|NotEqual(Enum) (Variables|Default|GetGameState) "NewEnumerator1")
        (Variables|Default|SetGameState "NewEnumerator1")
        (Development|PrintString "Ball Hit"))
      (CallFunction|LookatBall)
      (else
        (if (Utilities|Enum|Equal(Enum) (Variables|Default|GetGameState) "NewEnumerator1")
          (CallFunction|NewBall false))
        (if _biscurrentlypressed
          (if (Variables|Default|GetWasTouched)
            (Transformation|SetRelativeRotation _springarmcomponentline (Math|Rotator|MakeRotator (.roll _relativerotation) (.pitch _relativerotation) (+ (.yaw _relativerotation) (/ (- _locationx (Variables|Default|GetX)) (Variables|Default|GetCameraSpeed)))) false false)
            (Variables|Default|SetX _locationx)
            (Variables|Default|SetY _locationy)
            (else
              (Variables|Default|SetWasTouched true)
              (Variables|Default|SetX _locationx)
              (Variables|Default|SetY _locationy)))
          (CallFunction|MoveCamera)
          (if (Variables|/Script/GameAssignment.Golf_Ball|GetBallMoving (Variables|Default|GetGolfBall))
            (CallFunction|LookatBall))
          (else
            (Variables|Default|SetWasTouched false)))))))

(event Input|TouchEvents|InputTouch
  (params (Location :type Vector) (FingerIndex :type ETouchIndex%20Enum))
  (:Moved
    (Variables|Default|SetFinger FingerIndex)))

(fn ConstructionScript)