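; Game controller Blueprint that tracks elapsed level time and computes the final score from time and stroke count.
; Tick accumulates TimePassed from BeginPlay onward, without checking the Complete flag.
; LevelComplete sets Complete and calls CalcScore, which truncates a scaled ratio of time to Strokes, so longer times raise the score.
; Strokes is only read here.
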(event Custom|CalcScore
  ;[1 1 1] Calculates final score
  (Variables|Default|SetScore (Math|Float|Truncate (* (/ 1.0 (Math|Conversions|ToFloat(Integer) (Variables|Default|GetStrokes))) (Variables|Default|GetTimePassed) 135.0))))

(event Custom|LevelComplete
  (Variables|Default|SetComplete true)
  (CallFunction|CalcScore))

(event EventBeginPlay
  ;[1 1 1] Initial stuff
  (Variables|Default|SetTimePassed 0.0)
  (Variables|Default|SetComplete false))

(event Collision|EventActorBeginOverlap
  (params (OtherActor :type Actor%20Object%20Reference)))

(event EventTick
  (params (DeltaSeconds :type Float%20%28single-precision%29))
  (Variables|Default|SetTimePassed (+ DeltaSeconds (Variables|Default|GetTimePassed))))

(fn ConstructionScript)